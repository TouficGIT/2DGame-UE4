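; BP_PlatX is a moving platform actor that starts moving after a configurable delay.
; BeginPlay stores the actor's starting location, waits for the StartPlat delay, then sets a Start flag.
; While that flag is set, Tick calls Play on a timeline, whose track value is added to the stored location to reposition the platform without sweeping.
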(event `self.ReceiveBeginPlay`
  ;[1 1 1] Start Trigger Plat
  (set `self.locationOfPlat` (`self.K2_GetActorLocation`))
  (`KismetSystemLibrary.Delay` (`self.startPlat`))
  (set `self.start` true))

(event `self.ReceiveTick`
  (params (DeltaSeconds :type "Float (single-precision)"))
  ;[1 1 1] Add Plat Movement
  (if (`self.start`)
    (`|ExecutionSequence`
      (:`then_0`
        (bind (_direction _newtrack_0) (`Timeline|Timeline_0`)
          (:`Update`
            (`self.K2_SetActorLocation` (+ _newtrack_0 (`self.locationOfPlat`)))))))))

(fn `UserConstructionScript`)