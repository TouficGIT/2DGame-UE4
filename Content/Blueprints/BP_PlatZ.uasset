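; BP_PlatZ is a moving platform actor whose motion is driven by a timeline.
; BeginPlay caches the starting location, waits for a StartPlatZ delay, then sets the StartZ flag.
; While that flag is set, Tick calls Play on Timeline_PlatZ every frame, and each update sets the actor's location to the track value added to the cached start, without sweeping.
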(event `self.ReceiveBeginPlay`
  ;[1 1 1] Start Trigger Plat
  (set `self.location_of_platformZ` (`self.K2_GetActorLocation`))
  (`KismetSystemLibrary.Delay` (`self.StartPlatZ`))
  (set `self.startZ` true))

(event `self.ReceiveTick`
  (params (DeltaSeconds :type "Float (single-precision)"))
  ;[1 1 1] Add Plat Movement
  (if (`self.startZ`)
    (`|ExecutionSequence`
      (:`then_0`
        (bind (_direction _newtrack_0) (`Timeline|Timeline_PlatZ`)
          (:`Update`
            (`self.K2_SetActorLocation` (+ _newtrack_0 (`self.location_of_platformZ`)))))))))

(fn `UserConstructionScript`)