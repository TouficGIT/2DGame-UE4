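; BP_Turret is a sprite-based turret that automatically fires when the player is within range and can be destroyed by damage.
; Tick checks that the player is within a short X window on the turret's positive side and not too far above it, then triggers shooting.
; A DoOnce with a delayed reset limits the fire rate, spawning an actor at BulletArrow with a sound.
; DMG_Turret subtracts health, printing it until the turret is destroyed.
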(event `Turret_Shoot`
  ;[1 1 1] Turret Shooting
  (`/Engine/EditorBlueprintResources/StandardMacros.DoOnce` false :!label _label
    (:`Completed`
      (`|SpawnActorFromClass` "/Game/Blueprints/BP_TurretBullet.BP_TurretBullet_C" (`SceneComponent.K2_GetComponentToWorld` (`self.Bullet_Arrow`)) "Undefined" "OverrideRootScale" null null)
      (`GameplayStatics.PlaySound2D` "/Game/Sound/Game/Weapons/TurretBullet.TurretBullet" 0.8 1.0 0.0 null null)
      (`KismetSystemLibrary.Delay` 0.5)
      (goto _label :!via `Reset`))))

(event `self.ReceiveTick`
  (params (DeltaSeconds :type "Float (single-precision)"))
  (bind (_returnvalue_x _returnvalue_y _returnvalue_z) (`KismetMathLibrary.BreakVector` (`self.K2_GetActorLocation` (`GameplayStatics.GetPlayerCharacter` 0))))
  (bind (_returnvalue_x_2 _returnvalue_y_2 _returnvalue_z_2) (`KismetMathLibrary.BreakVector` (`SceneComponent.K2_GetComponentLocation` (`self.Sprite_turret`))))
  (bind _returnvalue (- _returnvalue_x_2 _returnvalue_x))
  ;[1 1 1] Distance Turret Start/Stop Shooting
  (if (<= _returnvalue 0.0)
    (if (<= (- _returnvalue_z _returnvalue_z_2) 50.0)
      (if (not (<= _returnvalue -500.0))
        (`self.Turret_Shoot`)))))

(event `DMG_Turret`
  (params (DMG_TurretTaken :type Integer))
  ;[1 1 1] Damage Turret System
  (bind _output_get (set `self.Turret_Health` (- (`self.Turret_Health`) DMG_TurretTaken)))
  (if (<= _output_get 0)
    (`self.K2_DestroyActor`)
    (else
      (`KismetSystemLibrary.PrintString` (`KismetStringLibrary.Conv_IntToString` (`self.Turret_Health`))))))

(fn `UserConstructionScript`)